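; First-person shooter character Blueprint that handles held-item attachment, camera effects and player appearance.
; Items attach to the first-person mesh for the local player, otherwise to the third-person mesh, which also takes them on ragdoll.
; Timelines blend per-weapon aiming FoV and smooth crouch eye height against capsule adjustment.
; Metadata drives team colour, materials and a cloak effect, while health events feed a post-process vignette showing health and damage direction.
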(event `self.OnEquippedUpdated`
  (params (NewHoldable :type "Holdable Object Reference"))
  ;[1 1 1] Attach weapon to correct mesh
  (`/Engine/EditorBlueprintResources/StandardMacros.IsValid` NewHoldable
    (:`Is Valid`
      (`self.K2_AttachToComponent` NewHoldable (select `bool` (`self.IsLocallyControlled`) :`false` (`self.Mesh`) :`true` (`self.FirstPersonMesh`)) (`Holdable.GetActiveSocket` NewHoldable) "SnapToTarget" "SnapToTarget" "KeepRelative" true))))

(event `self.StartRagdoll`
  (bind _returnvalue (`EquippedComponent.CurrentlyHeldItem` (`self.EquippedComponent`)))
  ;[1 1 1] Move equipped weapon to third person mesh on ragdoll
  (`parent.StartRagdoll`)
  (`/Engine/EditorBlueprintResources/StandardMacros.IsValid` _returnvalue
    (:`Is Valid`
      (`self.K2_AttachToComponent` _returnvalue (`self.Mesh`) (`Holdable.GetActiveSocket` _returnvalue) "SnapToTarget" "SnapToTarget" "KeepRelative" true))))

(event `self.GDKMovementComponent.OnAimingUpdated`
  (params (bIsAiming :type Boolean))
  (bind _firstpersoncamera (`self.FirstPersonCamera`))
  (bind _fieldofview (`CameraComponent.FieldOfView` (`self.FirstPersonCamera`)))
  ;[1 1 1] Aiming FoV
  (if bIsAiming
    (bind (_direction _fieldofview_2) (`Timeline|AimingFoV` :!label _label)
      (:`Update`
        (bind _asweapon (cast `Weapon` (`EquippedComponent.CurrentlyHeldItem` (`self.EquippedComponent`)))
          (:`then`
            (`CameraComponent.SetFieldOfView` _firstpersoncamera (`KismetMathLibrary.Lerp` (`self.DefaultFoV`) (select `ETimelineDirection` _direction :`Forward` (`Weapon.AimingFoV` _asweapon) :`Backward` _fieldofview) _fieldofview_2)))
          (:`CastFailed`
            (`CameraComponent.SetFieldOfView` _firstpersoncamera (`KismetMathLibrary.Lerp` (`self.DefaultFoV`) _fieldofview _fieldofview_2))))))
    (else
      (goto _label :!via `Reverse`))))

(event `self.K2_OnStartCrouch`
  (params (HalfHeightAdjust :type "Float (single-precision)") (ScaledHalfHeightAdjust :type "Float (single-precision)"))
  (bind _cachedeyeheight (`self.CachedEyeHeight`))
  (bind _firstpersoncamera (`self.FirstPersonCamera`))
  (bind _returnvalue (+ (`self.CrouchEyeHeightAdjustment`) _cachedeyeheight))
  (bind (_relativelocation_x _relativelocation_y) (`KismetMathLibrary.BreakVector` (`SceneComponent.RelativeLocation` _firstpersoncamera)))
  ;[1 1 1] Crouching
  (bind (_direction _croucheyeheightprogress) (`Timeline|CrouchTimeline` :!label _label_2)
    (:`Update`
      (`SceneComponent.K2_SetRelativeLocation` _firstpersoncamera (`KismetMathLibrary.MakeVector` _relativelocation_x _relativelocation_y (select `ETimelineDirection` _direction :`Forward` (`KismetMathLibrary.Lerp` (+ _cachedeyeheight HalfHeightAdjust) _returnvalue _croucheyeheightprogress) :`Backward` (`KismetMathLibrary.Lerp` (- _returnvalue HalfHeightAdjust) _cachedeyeheight (- 1.0 _croucheyeheightprogress)))) false false))))

(event `self.K2_OnEndCrouch`
  (params (HalfHeightAdjust :type "Float (single-precision)") (ScaledHalfHeightAdjust :type "Float (single-precision)"))
  ;[1 1 1] Crouching
  (goto _label_2 :!via `Reverse`))

(event `self.ReceiveBeginPlay`
  (bind _metadatacomponent (`self.MetaDataComponent`))
  (bind _meshmaterial (`self.MeshMaterial`))
  (bind _metadata_customization (break `GDKMetaData` (`MetaDataComponent.MetaData` _metadatacomponent)))
  (bind (_relativelocation_x _relativelocation_y _relativelocation_z) (`KismetMathLibrary.BreakVector` (`SceneComponent.RelativeLocation` (`self.FirstPersonCamera`))))
  (bind (_meta_data_index _meta_data_charactermaterial _meta_data_particlecolour) (break `/Game/Characters/MetaData/ColourDataRow` (`/Game/Characters/MetaData/MetaDataProvider.GetMetaData` (`self.MetaDataProvider`) _metadata_customization)))
  ;[1 1 1] BeginPlay
  (`parent.ReceiveBeginPlay`)
  (if (`self.IsLocallyControlled`)
    (`PrimitiveComponent.SetCollisionEnabled` (`self.Mesh`) "NoCollision"))
  ;[1 1 1] Cache Crouched Eye Height
  (set `self.CachedEyeHeight` _relativelocation_z)
  ;[1 1 1] Set Character Material based on MetaData component
  (if (`MetaDataComponent.bMetaDataAvailable` _metadatacomponent)
    (`MaterialInstanceDynamic.SetVectorParameterValue` (`self.NameplateMaterial`) "Team" _meta_data_particlecolour :!label _label_3)
    (bind _returnvalue (`PrimitiveComponent.CreateDynamicMaterialInstance` (`self.Mesh`) 0 _meta_data_charactermaterial "None"))
    (`/Engine/EditorBlueprintResources/StandardMacros.IsValid` _returnvalue
      (:`Is Valid`
        (set `self.MeshMaterial` _returnvalue)
        (`PrimitiveComponent.SetMaterial` (`self.FirstPersonMesh`) 0 null)
        (`MaterialInstanceDynamic.SetVectorParameterValue` _meshmaterial "Cloak_Colour" _meta_data_particlecolour)
        (bind (_direction _cloakoverride) (`Timeline|CloakTimeline`)
          (:`Update`
            (`MaterialInstanceDynamic.SetScalarParameterValue` _meshmaterial "Cloak_Override" _cloakoverride)))))))

(event `self.MetaDataComponent.MetaDataUpdated`
  (params (MetaData :type "GDKMetaData Structure"))
  ;[1 1 1] Set Character Material based on MetaData component
  (goto _label_3))

(event `self.HealthComponent.HealthUpdated`
  (params (Current :type "Float (single-precision)") (Max :type "Float (single-precision)"))
  ;[1 1 1] Health Vignette
  (`MaterialInstanceDynamic.SetScalarParameterValue` (`self.Vignette`) "Health" (/ Current Max))
  (`self.UpdateHealthMaterialValues` Current Max))

(event `self.HealthComponent.DamageTaken`
  (params (Value :type "Float (single-precision)") (Source :type "Vector Structure") (Impact :type "Vector Structure") (PlayerId :type Integer) (TeamId :type "GenericTeamId Structure"))
  (bind _vignette (`self.Vignette`))
  (bind _returnvalue (- Source (`self.K2_GetActorLocation`)))
  ;[1 1 1] Damage Indicator
  (`MaterialInstanceDynamic.SetScalarParameterValue` _vignette "Damage_Focus" (`KismetMathLibrary.MapRangeClamped` (`KismetMathLibrary.VSize` _returnvalue) 0.0 100.0 25.0 15.0))
  (bind (_direction _intensity) (`Timeline|ImpactIntensity` :!via `PlayFromStart`)
    (:`Update`
      (`MaterialInstanceDynamic.SetScalarParameterValue` _vignette "Damage_Intensity" _intensity)
      (`MaterialInstanceDynamic.SetScalarParameterValue` _vignette "Damage_Yaw" (- (`KismetMathLibrary.GetYawPitchFromVector` _returnvalue) (`KismetMathLibrary.GetYawPitchFromVector` (`self.GetActorForwardVector`)))))))

(fn `UserConstructionScript`
  (`parent.UserConstructionScript`)
  (bind _returnvalue (`KismetMaterialLibrary.CreateDynamicMaterialInstance` "/Game/Base/PostMaterials/M_Post_DirectionalDamageVignette.M_Post_DirectionalDamageVignette"))
  (bind _output_get (set `self.Vignette` _returnvalue))
  (`MaterialInstanceDynamic.SetScalarParameterValue` _output_get "Health" 1.0)
  (`CameraComponent.AddOrUpdateBlendable` (`self.FirstPersonCamera`) _output_get 1.0))